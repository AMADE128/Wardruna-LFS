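; HDRI environment actor that sets up sky, lighting, fog and post-processing from exposed variables, entirely in the construction script.
; One HDR texture feeds both the SkyLight cubemap and a dynamic material on the sky sphere, with separate light intensity and sky brightness controls.
; It also sets post-process bloom, saturation and exposure, plus exponential height fog density, falloff, color, opacity and start distance.
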(event EventBeginPlay)

(event Collision|EventActorBeginOverlap
  (params (OtherActor :type Actor%20Object%20Reference)))

(event EventTick
  (params (DeltaSeconds :type Float%20%28single-precision%29)))

(fn ConstructionScript
  (bind _exponentialheightfog (Variables|Default|GetExponentialHeightFog))
  (bind _skylight (Variables|Default|GetSkyLight))
  (Rendering|SetVisibility (Variables|Default|GetSkyLight) false false)
  (Class|SkyLightComponent|SetCubemap _skylight (Variables|MainHDR|GetHDRTexture))
  (Rendering|Components|Light|SetIntensity _skylight (Variables|MainHDR|GetSkylightIntensity))
  (Rendering|SetVisibility (Variables|Default|GetSkyLight) true false)
  (Utilities|IsValid (Variables|MainHDR|GetHDR_Material)
    (:Is%20Valid
      _)
    (:Is%20Not%20Valid
      (bind _returnvalue (Rendering|Material|CreateDynamicMaterialInstance (Variables|Default|GetSM_SkySphere) 0 "/Game/Contents/HDRI/belfast_sunset_puresky_4k_Mat.belfast_sunset_puresky_4k_Mat" "None" :!class /Script/Engine.PrimitiveComponent))
      (Variables|MainHDR|SetHDR_Material _returnvalue)))
  (Rendering|Material|SetTextureParameterValue (Variables|MainHDR|GetHDR_Material) "SkyParameter" (Variables|MainHDR|GetHDRTexture))
  (Rendering|Material|SetScalarParameterValue (Variables|MainHDR|GetHDR_Material) "SkyBrightness" (Variables|MainHDR|GetSkyTextureBrightness) :!class /Script/Engine.MaterialInstanceDynamic)
  (Utilities|Struct|SetmembersinPostProcessSettings (Variables|/Script/Engine.PostProcessComponent|GetSettings (Variables|Default|GetPostProcess)) (Variables|PostProcess|GetMethod) (Variables|PostProcess|GetSaturation) (Variables|PostProcess|GetIntensity) (Variables|PostProcess|GetSize%20Scale) (Variables|PostProcess|Get#%201%20Size) (Variables|PostProcess|Get#%201%20Tint) (Variables|PostProcess|GetExposure%20Compensation) (Variables|PostProcess|GetMin%20EV100) (Variables|PostProcess|GetMax%20EV100))
  (Class|ExponentialHeightFogComponent|SetFogDensity _exponentialheightfog (Variables|Fog|GetFogDensity))
  (Class|ExponentialHeightFogComponent|SetFogHeightFalloff _exponentialheightfog (Variables|Fog|GetFogFalloff))
  (Class|ExponentialHeightFogComponent|SetFogInscatteringColor _exponentialheightfog (* (Variables|Fog|GetFogColor) (Variables|Fog|GetColorIntensity)))
  (Class|ExponentialHeightFogComponent|SetFogMaxOpacity _exponentialheightfog (Variables|Fog|GetMaxOpacity))
  (Class|ExponentialHeightFogComponent|SetStartDistance _exponentialheightfog (Variables|Fog|GetFogDistance)))