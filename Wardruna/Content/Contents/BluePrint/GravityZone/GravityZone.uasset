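; Gravity zone actor that turns the player's gravity off on begin overlap and restores it to normal on end overlap, printing a message each time.
; Both overlap events set the movement GravityScale of player 0's BP_FirstPersonCharacter, whichever actor triggered them.
; The construction script configures an InteractChildActor from ChildConfig and scales CollisionGravedad by ZoneRadius.
; A FlipFlop toggle between both gravity states is left unconnected.
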(event EventBeginPlay)

(event Collision|EventActorBeginOverlap
  (params (OtherActor :type Actor%20Object%20Reference))
  (bind _returnvalue (Game|GetPlayerCharacter 0))
  (bind (_asbp_first_person_character _bsuccess) (Utilities|Casting|CastToBP_FirstPersonCharacter _returnvalue))
  (if _bsuccess
    (Variables|/Script/Engine.CharacterMovementComponent|SetGravityScale (Variables|/Script/Engine.Character|GetCharacterMovement _asbp_first_person_character) 0.0)
    (Development|PrintText "Gravedad a 0!")))

(event EventTick
  (params (DeltaSeconds :type Float%20%28single-precision%29)))

(event Collision|EventActorEndOverlap
  (params (OtherActor :type Actor%20Object%20Reference))
  (bind _returnvalue (Game|GetPlayerCharacter 0))
  (bind (_asbp_first_person_character _bsuccess) (Utilities|Casting|CastToBP_FirstPersonCharacter _returnvalue))
  (if _bsuccess
    (Variables|/Script/Engine.CharacterMovementComponent|SetGravityScale (Variables|/Script/Engine.Character|GetCharacterMovement _asbp_first_person_character) 1.0)
    (Development|PrintText "Gravedad NORMAL!")))

(fn ConstructionScript
  (|CoroConstruct_2_2 (Variables|Default|GetChildActor) (Variables|Default|GetChildConfig)))