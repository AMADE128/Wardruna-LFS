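; Markus NPC that starts a dialogue when its ActivarObjeto event fires, passing its SKMManny mesh to the dialogue component.
; The construction script applies the ChildConfig struct to an InteractChildActor child actor through CoroConstruct_2_2.
; That function sets the interaction text, icon material, sphere and box trigger sizes, once-only flag and initial active state, so the prompt is configured from the parent.
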(event EventActivarObjeto
  (Default|ActivarDialogo (Variables|Default|GetBP_DialogueComponent) (Variables|Default|GetSKM_Manny)))

(fn ConstructionScript
  (|CoroConstruct_2_2 (Variables|Default|GetChildActor) (Variables|Default|GetChildConfig)))