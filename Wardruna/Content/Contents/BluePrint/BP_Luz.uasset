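; BP_Luz is an interactable light whose ActivarObjeto event alternately hides and shows its point light through a FlipFlop, hiding it on the first call.
; The construction script passes ChildConfig and its ChildActor component to CoroConstruct_2.
; That graph casts the child to InteractChildActor and copies in prompt text, sphere and trigger sizes, once-only and starting-active flags, and icon material, so each instance configures its own interaction.
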(event EventActivarObjeto
  (Utilities|FlowControl|FlipFlop
    (:A
      (Development|SetHiddeninGame (Variables|Default|GetPointLight) true false))
    (:B
      (Development|SetHiddeninGame (Variables|Default|GetPointLight) false false))))

(fn ConstructionScript
  (|CoroConstruct_2 (Variables|Default|GetChildActor) (Variables|Default|GetChildConfig)))