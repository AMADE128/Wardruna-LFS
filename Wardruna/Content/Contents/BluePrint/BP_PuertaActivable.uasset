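; BP_PuertaActivable is an activatable door that toggles between raised and lowered positions.
; Each ActivarObjeto event alternately plays or reverses a timeline that lerps the Scene component's relative height.
; The construction script pushes ChildConfig into an InteractChildActor child actor, setting its prompt text, icon, trigger shapes, do-once flag and initial active state.
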(event EventBeginPlay)

(event Collision|EventActorBeginOverlap
  (params (OtherActor :type Actor%20Object%20Reference)))

(event EventTick
  (params (DeltaSeconds :type Float%20%28single-precision%29)))

(event EventActivarObjeto
  (Utilities|FlowControl|FlipFlop
    (:A
      (bind _newtrack_0 (Timeline|AnimacionPuerta Play)
        (:Update
          (Transformation|SetRelativeLocation (Variables|Default|GetScene) (Math|Vector|MakeVector 0.0 0.0 (Math|Float|Lerp 0.0 2e+02 _newtrack_0)) false false))))
    (:B
      (Timeline|AnimacionPuerta Reverse))))

(fn ConstructionScript
  (|CoroConstruct_2 (Variables|Default|GetChildActor) (Variables|Default|GetChildConfig)))