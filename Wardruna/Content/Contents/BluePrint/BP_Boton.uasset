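; BP_Boton is an interactable button that activates a referenced object through a message call.
; ActivarObjeto messages ObjetoAActivar, fires the ButtonActivated dispatcher, then dips the cube briefly while disabling its InteractChildActor until the cube rises again.
; The construction script passes ChildConfig to CoroConstruct, which configures that child actor's prompt text, icon, trigger sizes, one-use flag and initial active state.
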(event EventBeginPlay)

(event Collision|EventActorBeginOverlap
  (params (OtherActor :type Actor%20Object%20Reference)))

(event EventTick
  (params (DeltaSeconds :type Float%20%28single-precision%29)))

(event EventActivarObjeto
  (Class|InteractBlueprintInterface|ActivarObjeto(Message) (Variables|Default|GetObjetoAActivar))
  (Default|CallButtonActivatedDispatched)
  (Transformation|AddLocalOffset (Variables|Default|GetCube) "0.000000,0.000000,-10.000000" false false)
  (Default|DesableInteract (.AsInteract%20Child%20Actor (Utilities|Casting|CastToInteractChildActor (Variables|/Script/Engine.ChildActorComponent|GetChildActor (Variables|Default|GetChildActor)))))
  (Utilities|FlowControl|Delay 0.2)
  (Transformation|AddLocalOffset (Variables|Default|GetCube) "0.000000,0.000000,10.000000" false false)
  (Default|EnableInteract (.AsInteract%20Child%20Actor (Utilities|Casting|CastToInteractChildActor (Variables|/Script/Engine.ChildActorComponent|GetChildActor (Variables|Default|GetChildActor))))))

(fn ConstructionScript
  (|CoroConstruct (Variables|Default|GetChildActor) (Variables|Default|GetChildConfig)))