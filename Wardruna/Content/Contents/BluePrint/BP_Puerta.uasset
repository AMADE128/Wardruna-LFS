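; Interactable door Blueprint that swings open and closed around a hinge scene component.
; ActivarObjeto flip-flops a timeline forward and in reverse, lerping the hinge's yaw.
; Each timeline update also disables the InteractChildActor's interaction, with a short delay before re-enabling it.
; The construction script copies ChildConfig into that child actor, setting its prompt text, icon, trigger sizes, do-once and initial active state.
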(event EventBeginPlay)

(event Collision|EventActorBeginOverlap
  (params (OtherActor :type Actor%20Object%20Reference)))

(event EventTick
  (params (DeltaSeconds :type Float%20%28single-precision%29)))

(event EventActivarObjeto
  (Utilities|FlowControl|FlipFlop
    (:A
      (bind _newtrack_0 (Timeline|AnimacionPuerta Play)
        (:Update
          (Transformation|SetRelativeRotation (Variables|Default|GetScene) (Math|Rotator|MakeRotator 0.0 0.0 (Math|Float|Lerp 0.0 -85.0 _newtrack_0)) false false)
          (Default|DesableInteract (.AsInteract%20Child%20Actor (Utilities|Casting|CastToInteractChildActor (Variables|/Script/Engine.ChildActorComponent|GetChildActor (Variables|Default|GetChildActor)))))
          (Utilities|FlowControl|Delay 1.5)
          (Default|EnableInteract (.AsInteract%20Child%20Actor (Utilities|Casting|CastToInteractChildActor (Variables|/Script/Engine.ChildActorComponent|GetChildActor (Variables|Default|GetChildActor))))))))
    (:B
      (Timeline|AnimacionPuerta Reverse))))

(fn ConstructionScript
  (|CoroConstruct_2 (Variables|Default|GetChildActor) (Variables|Default|GetChildConfig)))